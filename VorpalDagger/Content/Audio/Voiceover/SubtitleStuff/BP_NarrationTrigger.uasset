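; BP_NarrationTrigger is a one-shot trigger volume that plays a narration level sequence when BP_VorpalDaggerController overlaps it.
; On overlap it disables its collision and finds the BP_NarrationManager among actors tagged "Narration".
; It calls the manager's ChangeSequence with the game mode's current narration player and its own sequence actor.
; It creates an auto-playing player for its Narration sequence and destroys itself after that sequence's duration.
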(event OnComponentBeginOverlap(CollisionComponent)
  (params (OverlappedComponent :type Primitive%20Component%20Object%20Reference) (OtherActor :type Actor%20Object%20Reference) (OtherComp :type Primitive%20Component%20Object%20Reference) (OtherBodyIndex :type Integer) (bFromSweep :type Boolean) (SweepResult :type Hit%20Result%20Structure%20%28by%20ref%29))
  (Utilities|Casting|CastToBP_VorpalDaggerController OtherActor)
  (Collision|SetCollisionEnabled (Variables|Default|GetCollisionComponent) "NoCollision")
  (bind _outactors (Actor|GetAllActorswithTag "Narration"))
  (for _array_element _outactors
    (bind _asbp_narration_manager (Utilities|Casting|CastToBP_NarrationManager _array_element))
    (bind _asgm_vorpal_dagger (Utilities|Casting|CastToGM_VorpalDagger (Game|GetGameMode)))
    (Default|ChangeSequence _asbp_narration_manager (Variables|/Game/ThirdPersonBP/Blueprints/GM_VorpalDagger.GM_VorpalDagger_C|GetCurrentNarrationPlayer _asgm_vorpal_dagger) (stale _outactor))
    (bind (_outactor _returnvalue) (Sequencer|Player|CreateLevelSequencePlayer (Variables|Default|GetNarration) (Utilities|Struct|MakeMovieSceneSequencePlaybackSettings true "(Value=0)" 1.0 0.0 false false false false false false false false)))
    (Utilities|FlowControl|Delay (Class|TimeManagementBlueprintLibrary|ToSeconds(QualifiedFrameTime) (Media|MediaPlayer|GetDuration _returnvalue)))
    (Actor|DestroyActor)))

(event EventBeginPlay)

(event Collision|EventActorBeginOverlap
  (params (OtherActor :type Actor%20Object%20Reference)))

(event EventTick
  (params (DeltaSeconds :type Float%20%28single-precision%29)))

(fn ConstructionScript)