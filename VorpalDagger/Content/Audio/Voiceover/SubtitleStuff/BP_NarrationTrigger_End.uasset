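; One-shot narration trigger that plays the good, mild or bad ending when BP_VorpalDaggerController overlaps it.
; It passes the game mode's current narration player to the tagged BP_NarrationManager's ChangeSequence, then branches on score.
; Exactly 1000 gives good, nonzero up to 500 gives mild, and anything else, including 501–999, gives bad.
; Each ending chains Level Sequences through duration-based Delays, then destroys the trigger.
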(event OnComponentBeginOverlap(CollisionComponent)
  (params (OverlappedComponent :type Primitive%20Component%20Object%20Reference) (OtherActor :type Actor%20Object%20Reference) (OtherComp :type Primitive%20Component%20Object%20Reference) (OtherBodyIndex :type Integer) (bFromSweep :type Boolean) (SweepResult :type Hit%20Result%20Structure%20%28by%20ref%29))
  (Collision|SetCollisionEnabled (Variables|Default|GetCollisionComponent) "NoCollision")
  (Utilities|Casting|CastToBP_VorpalDaggerController OtherActor)
  (bind _asgm_vorpal_dagger (Utilities|Casting|CastToGM_VorpalDagger (Game|GetGameMode)))
  (bind _score (Default|GetScore _asgm_vorpal_dagger))
  (bind _outactors (Actor|GetAllActorswithTag "Narration"))
  (for _array_element _outactors
    (bind _asbp_narration_manager (Utilities|Casting|CastToBP_NarrationManager _array_element))
    (bind _asgm_vorpal_dagger_2 (Utilities|Casting|CastToGM_VorpalDagger (Game|GetGameMode)))
    (Default|ChangeSequence _asbp_narration_manager (Variables|/Game/ThirdPersonBP/Blueprints/GM_VorpalDagger.GM_VorpalDagger_C|GetCurrentNarrationPlayer _asgm_vorpal_dagger_2))
    (if (== _score 1000)
      (bind _outactor (Sequencer|Player|CreateLevelSequencePlayer "/Game/Audio/Voiceover/SubtitleStuff/NLS_stuff/NLS_GoodEndingPart1.NLS_GoodEndingPart1" (Utilities|Struct|MakeMovieSceneSequencePlaybackSettings true "(Value=0)" 1.0 0.0 false false false false false false false false)))
      (Utilities|FlowControl|Delay (Class|TimeManagementBlueprintLibrary|ToSeconds(QualifiedFrameTime) (Media|MediaPlayer|GetDuration (Variables|/Script/LevelSequence.LevelSequenceActor|GetSequencePlayer _outactor))))
      (bind _outactor_2 (Sequencer|Player|CreateLevelSequencePlayer "/Game/Audio/Voiceover/SubtitleStuff/NLS_stuff/NLS_GoodEndingPart2.NLS_GoodEndingPart2" (Utilities|Struct|MakeMovieSceneSequencePlaybackSettings true "(Value=0)" 1.0 0.0 false false false false false false false false)))
      (Utilities|FlowControl|Delay (Class|TimeManagementBlueprintLibrary|ToSeconds(QualifiedFrameTime) (Media|MediaPlayer|GetDuration (Variables|/Script/LevelSequence.LevelSequenceActor|GetSequencePlayer _outactor_2))))
      (Actor|DestroyActor)
      (elif (and (<= _score 500) (!= _score 0))
        (bind _outactor_3 (Sequencer|Player|CreateLevelSequencePlayer "/Game/Audio/Voiceover/SubtitleStuff/NLS_stuff/NLS_MildEndingPart1.NLS_MildEndingPart1" (Utilities|Struct|MakeMovieSceneSequencePlaybackSettings true "(Value=0)" 1.0 0.0 false false false false false false false false)))
        (Utilities|FlowControl|Delay (Class|TimeManagementBlueprintLibrary|ToSeconds(QualifiedFrameTime) (Media|MediaPlayer|GetDuration (Variables|/Script/LevelSequence.LevelSequenceActor|GetSequencePlayer _outactor_3))))
        (bind _outactor_4 (Sequencer|Player|CreateLevelSequencePlayer "/Game/Audio/Voiceover/SubtitleStuff/NLS_stuff/NLS_MildEndingPart2.NLS_MildEndingPart2" (Utilities|Struct|MakeMovieSceneSequencePlaybackSettings true "(Value=0)" 1.0 0.0 false false false false false false false false)))
        (Utilities|FlowControl|Delay (Class|TimeManagementBlueprintLibrary|ToSeconds(QualifiedFrameTime) (Media|MediaPlayer|GetDuration (Variables|/Script/LevelSequence.LevelSequenceActor|GetSequencePlayer _outactor_4))))
        (Actor|DestroyActor)
        (else
          (bind _outactor_5 (Sequencer|Player|CreateLevelSequencePlayer "/Game/Audio/Voiceover/SubtitleStuff/NLS_stuff/NLS_BadEndingPart1.NLS_BadEndingPart1" (Utilities|Struct|MakeMovieSceneSequencePlaybackSettings true "(Value=0)" 1.0 0.0 false false false false false false false false)))
          (Utilities|FlowControl|Delay (Class|TimeManagementBlueprintLibrary|ToSeconds(QualifiedFrameTime) (Media|MediaPlayer|GetDuration (Variables|/Script/LevelSequence.LevelSequenceActor|GetSequencePlayer _outactor_5))))
          (bind _outactor_6 (Sequencer|Player|CreateLevelSequencePlayer "/Game/Audio/Voiceover/SubtitleStuff/NLS_stuff/NLS_BadEndingPart2.NLS_BadEndingPart2" (Utilities|Struct|MakeMovieSceneSequencePlaybackSettings true "(Value=0)" 1.0 0.0 false false false false false false false false)))
          (Utilities|FlowControl|Delay (Class|TimeManagementBlueprintLibrary|ToSeconds(QualifiedFrameTime) (Media|MediaPlayer|GetDuration (Variables|/Script/LevelSequence.LevelSequenceActor|GetSequencePlayer _outactor_6))))
          (bind _outactor_7 (Sequencer|Player|CreateLevelSequencePlayer "/Game/Audio/Voiceover/SubtitleStuff/NLS_stuff/NLS_BadEndingPart3.NLS_BadEndingPart3" (Utilities|Struct|MakeMovieSceneSequencePlaybackSettings true "(Value=0)" 1.0 0.0 false false false false false false false false)))
          (Utilities|FlowControl|Delay (Class|TimeManagementBlueprintLibrary|ToSeconds(QualifiedFrameTime) (Media|MediaPlayer|GetDuration (Variables|/Script/LevelSequence.LevelSequenceActor|GetSequencePlayer _outactor_7))))
          (Actor|DestroyActor))))))

(fn ConstructionScript
  (|CallParentFunction))