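; BP_NumberedRune is a hittable rune object with an order number, an active state, a destructible flag and a point modifier.
; Its Hit event toggles the active state and prints the order number when turning on, using a DoOnce gate that resets after a short delay to debounce repeated hits.
; Getter functions expose the rune's properties, and a setter lets other code override the active state.
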(event Collision|EventHit
  (params (MyComp :type Primitive%20Component%20Object%20Reference) (Other :type Actor%20Object%20Reference) (OtherComp :type Primitive%20Component%20Object%20Reference) (bSelfMoved :type Boolean) (HitLocation :type Vector :default "0, 0, 0") (HitNormal :type Vector :default "0, 0, 0") (NormalImpulse :type Vector :default "0, 0, 0") (Hit :type Hit%20Result%20Structure%20%28by%20ref%29))
  (Utilities|FlowControl|DoOnce false :!label _label
    (:Completed
      (if (Variables|Default|GetActiveState)
        (Variables|Default|SetActiveState false)
        (Utilities|FlowControl|Delay 0.2)
        (goto _label Reset)
        (else
          (Variables|Default|SetActiveState true)
          (Development|PrintString (Utilities|String|ToString(Integer) (Variables|Default|GetOrderNumber)))
          (Utilities|FlowControl|Delay 0.2)
          (goto _label Reset))))))

(fn ConstructionScript)

(fn GetActiveState
  (return (Variables|Default|GetActiveState)))

(fn GetDestructable
  (return (Variables|Default|GetDestructable)))

(fn GetOrderNumber
  (return (Variables|Default|GetOrderNumber)))

(fn GetPointMod
  (return (Variables|Default|GetPointMod)))

(fn SetActiveState
  (params (SetInactive :type Boolean))
  (bind _output_get (Variables|Default|SetActiveState SetInactive))
  (return _output_get))