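; BP_DestructableRune is a rune actor that is removed when it receives a Hit event.
; Hit sets its ActiveState to false, then destroys the actor.
; Getter functions expose the active state, the destructable flag and a point modifier, while the order number always returns zero.
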(event Collision|EventHit
  (params (MyComp :type Primitive%20Component%20Object%20Reference) (Other :type Actor%20Object%20Reference) (OtherComp :type Primitive%20Component%20Object%20Reference) (bSelfMoved :type Boolean) (HitLocation :type Vector :default "0, 0, 0") (HitNormal :type Vector :default "0, 0, 0") (NormalImpulse :type Vector :default "0, 0, 0") (Hit :type Hit%20Result%20Structure%20%28by%20ref%29))
  (CallFunction|SetActiveState false)
  (Actor|DestroyActor))

(fn ConstructionScript)

(fn GetActiveState
  (return (Variables|Default|GetActiveState)))

(fn GetDestructable
  (return (Variables|Default|GetDestructable)))

(fn GetOrderNumber
  (return 0))

(fn GetPointMod
  (return (Variables|Default|GetPointMod)))

(fn SetActiveState
  (params (SetInactive :type Boolean))
  (bind _output_get (Variables|Default|SetActiveState SetInactive))
  (return _output_get))