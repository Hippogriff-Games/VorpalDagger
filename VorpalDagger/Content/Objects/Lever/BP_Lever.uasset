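; BP_Lever is a lever object that flips between two states when it receives a Hit event.
; Each hit inverts LeverState and rotates LeverMesh one way or the other by a fixed relative step.
; A DoOnce gate, reset after a short delay, blocks repeat hits during that window.
; GetLeverState, GetDestructable and GetPointMod all return a constant false, so GetLeverState does not report the stored state.
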(event Collision|EventHit
  (params (MyComp :type Primitive%20Component%20Object%20Reference) (Other :type Actor%20Object%20Reference) (OtherComp :type Primitive%20Component%20Object%20Reference) (bSelfMoved :type Boolean) (HitLocation :type Vector :default "0, 0, 0") (HitNormal :type Vector :default "0, 0, 0") (NormalImpulse :type Vector :default "0, 0, 0") (Hit :type Hit%20Result%20Structure%20%28by%20ref%29))
  (Utilities|FlowControl|DoOnce false :!label _label
    (:Completed
      (bind _notleverstate (CallFunction|ToggleLeverState (Variables|Default|GetLeverState)))
      (bind _output_get (Variables|Default|SetLeverState _notleverstate))
      (if _output_get
        (Transformation|AddRelativeRotation (Variables|Default|GetLeverMesh) "35.000000,0.000000,0.000000" false false)
        (Utilities|FlowControl|Delay 0.5)
        (goto _label Reset)
        (else
          (Transformation|AddRelativeRotation (Variables|Default|GetLeverMesh) "-35.000000,0.000000,0.000000" false false)
          (Utilities|FlowControl|Delay 0.5)
          (goto _label Reset))))))

(fn ConstructionScript)

(fn GetDestructable
  (return false))

(fn GetLeverState
  (return false))

(fn GetPointMod
  (return false))

(fn ToggleLeverState
  (params (LeverState :type Boolean))
  (return (not LeverState)))