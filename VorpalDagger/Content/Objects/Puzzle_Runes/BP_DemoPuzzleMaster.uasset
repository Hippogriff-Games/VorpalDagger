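; BP_DemoPuzzleMaster is a rune puzzle controller that destroys itself once all of its tracked runes are destroyed.
; On BeginPlay it binds to the DestroyRune dispatcher of the runes in its DestructRunes array.
; Each dispatch passes the destroyed rune to ProgressPuzzle, which removes it from the array and calls DestroyPuzzle when none remain.
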(event Custom|DestroyRune_Event_0
  (params (NewParam :type BP%20Destructable%20Rune%20Object%20Reference))
  (CallFunction|ProgressPuzzle NewParam))

(event EventBeginPlay
  (EventDispatchers|AssignDestroyRune (Variables|Default|GetDestructRunes) (delegate Custom|DestroyRune_Event_0)))

(fn ConstructionScript)

(fn ProgressPuzzle
  (params (DestroyedRune :type BP%20Destructable%20Rune%20Object%20Reference))
  (bind _destructrunes (Variables|Default|GetDestructRunes))
  (Utilities|Array|RemoveItem _destructrunes DestroyedRune)
  (if (not (> (Utilities|Array|Length _destructrunes) 0))
    (CallFunction|DestroyPuzzle)))

(fn DestroyPuzzle
  (Actor|DestroyActor))