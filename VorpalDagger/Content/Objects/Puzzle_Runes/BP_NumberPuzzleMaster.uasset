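; Puzzle master actor for a rune number puzzle in which runes must be triggered in ascending order.
; On BeginPlay it binds to the UpdatePuzzle dispatcher on its referenced Runes, passing each reported order number to ProgressPuzzle.
; A correct number advances the expected value until it reaches End, destroying the runes and the master.
; A wrong number deactivates all runes, makes them visible and restarts the count at one.
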(event Custom|CustomEvent_1
  (params (OrderNumber :type Integer))
  (CallFunction|ProgressPuzzle OrderNumber))

(event EventBeginPlay
  (EventDispatchers|AssignUpdatePuzzle (Variables|Default|GetRunes) (delegate Custom|CustomEvent_1)))

(fn ConstructionScript)

(fn ProgressPuzzle
  (params (RuneNum :type Integer))
  (if (== RuneNum (Variables|Default|GetExpectedNext))
    (bind _output_get (Variables|Default|SetExpectedNext (+ (Variables|Default|GetExpectedNext) 1)))
    (if (== _output_get (Variables|Default|GetEnd))
      (CallFunction|DestroyPuzzle))
    (else
      (CallFunction|ResetPuzzle))))

(fn ResetPuzzle
  (for _array_element (Variables|Default|GetRunes)
    (Default|SetActiveState _array_element false)
    (Rendering|SetVisibility (Variables|/Script/Engine.Actor|GetRootComponent _array_element) true false))
  (Variables|Default|SetExpectedNext 1))

(fn DestroyPuzzle
  (for _array_element (Variables|Default|GetRunes)
    (Actor|DestroyActor _array_element))
  (Actor|DestroyActor))