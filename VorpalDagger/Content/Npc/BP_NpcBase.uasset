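; Base NPC character that can chase the player, exposes a patrol route and dies on capsule impact.
; Any valid actor hitting the capsule destroys it and triggers Death, which ragdolls the mesh, disables movement and destroys the actor after a delay.
; Chaseplayer uses AI MoveTo toward the player and re-calls itself after a delay only on success.
; SetMovementSpeed maps a speed state to max walk speed.
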(event OnComponentHit(CapsuleComponent)
  (params (HitComponent :type Primitive%20Component%20Object%20Reference) (OtherActor :type Actor%20Object%20Reference) (OtherComp :type Primitive%20Component%20Object%20Reference) (NormalImpulse :type Vector :default "0, 0, 0") (Hit :type Hit%20Result%20Structure%20%28by%20ref%29))
  (Utilities|IsValid OtherActor
    (:Is%20Valid
      (Components|DestroyComponent (Variables|Default|GetCapsuleComponent))
      (CallFunction|Death))
    (:Is%20Not%20Valid
      (Development|PrintString "Not valid"))))

(event Custom|Death
  (Physics|SetSimulatePhysics (Variables|Character|GetMesh) true)
  (Pawn|Components|CharacterMovement|DisableMovement (Variables|Character|GetCharacterMovement))
  (Utilities|FlowControl|Delay 3.0)
  (Actor|DestroyActor))

(event Custom|Chase%20player
  (AI|AIMoveTo self "0, 0, 0" (Game|GetPlayerCharacter 0) 1.5e+02 false
    (:OnSuccess
      (Utilities|FlowControl|Delay 3.0)
      (CallFunction|ChasePlayer))))

(event EventBeginPlay)

(fn ConstructionScript)

(fn GetPatrolRoute
  (return (Variables|AI|GetPatrolRoute)))

(fn SetMovementSpeed
  (params (Speed :type E_MovementSpeed%20Enum :default "NewEnumerator0"))
  (bind _output_get (Variables|/Script/Engine.CharacterMovementComponent|SetMaxWalkSpeed (Variables|Character|GetCharacterMovement) (Utilities|Select :Index Speed :NewEnumerator0 0.0 :NewEnumerator1 1e+02 :NewEnumerator2 3e+02 :NewEnumerator3 5e+02)))
  (return _output_get))